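; BP_CheckpointFlag is a checkpoint flag that sets the player's respawn point when an actor overlaps it.
; On overlap it deactivates every active checkpoint in the GS_DES250 game state's Checkpoints list, plays a bell sound, and activates itself, swapping the flag wedge material to show state.
; It then writes its location and rotation to player 0's AC_Health component, without checking which actor overlapped.
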(event `self.ReceiveActorBeginOverlap`
  (params (OtherActor :type "Actor Object Reference"))
  (`self.DeactivateAll`)
  (`GameplayStatics.PlaySound2D` "/Game/DoNotChange/PrototypingAssets/Sounds/GeneralFeedback/DES_SFX_Bell_01.DES_SFX_Bell_01" 1.0 1.0 0.0 null null)
  (`self.Activate`)
  (`self.UpdateRespawn`))

(fn `Activate`
  (set `self.IsActive` true)
  (`PrimitiveComponent.SetMaterial` (`self.FlagWedge`) 0 "/Game/Material_009.Material_009"))

(fn `Deactivate`
  (set `self.IsActive` false)
  (`PrimitiveComponent.SetMaterial` (`self.FlagWedge`) 0 "/Game/Assets/Material_007.Material_007"))

(fn `DeactivateAll`
  (bind _asgs_des250 (cast `/Game/GameModes/GS_DES250` (`GameplayStatics.GetGameState`)))
  (for _array_element (`/Game/GameModes/GS_DES250.Checkpoints` _asgs_des250)
    (if (`/Game/GameplayBlueprints/BP_CheckpointFlag.IsActive` _array_element)
      (`self.Deactivate` _array_element)))
  (return))

(fn `UpdateRespawn`
  (bind _returnvalue (`self.GetComponentByClass` (`GameplayStatics.GetPlayerPawn` 0) "/Game/ActorComponents/AC_Health.AC_Health_C"))
  (`/Engine/EditorBlueprintResources/StandardMacros.IsValid` _returnvalue
    (:`Is Valid`
      (set `/Game/ActorComponents/AC_Health.RespawnLocation` (`self.K2_GetActorLocation`) _returnvalue)
      (set `/Game/ActorComponents/AC_Health.RespawnRotation` (`self.K2_GetActorRotation`) _returnvalue))))

(fn `UserConstructionScript`)