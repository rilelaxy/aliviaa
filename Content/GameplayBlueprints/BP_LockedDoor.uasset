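; BP_LockedDoor is an interactable door that opens only when the player's inventory holds a key.
; Player overlap shows the FrontWidget prompt and enables E input; leaving reverses both.
; With a key, E consumes it, plays a sound, hides the widget and trigger, disables DoorFrame collision, and rotates Door yaw through a Timeline.
; Without a key, E plays a deny sound.
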(event `Key|E`
  (params (Key :type "Key Structure"))
  (:`Pressed`
    (if (`self.PlayerHasKey`)
      (`self.OpenDoor`)
      (bind (_direction _doorrotation) (`Timeline|Timeline`)
        (:`Update`
          (`SceneComponent.K2_SetRelativeRotation` (`self.Door`) (`KismetMathLibrary.MakeRotator` 0.0 0.0 _doorrotation) false false)))
      (else
        (`GameplayStatics.PlaySound2D` "/Game/DoNotChange/PrototypingAssets/Sounds/GeneralFeedback/DES_SFX_Deny_05.DES_SFX_Deny_05" 1.0 1.0 0.0 null null)))))

(event `self.ReceiveActorBeginOverlap`
  (params (OtherActor :type "Actor Object Reference"))
  (`/Game/DES250_Macros.PlayerCheck` OtherActor
    (:`IsPlayer`
      (`SceneComponent.SetVisibility` (`self.FrontWidget`) true false)
      (`self.EnableInput` (`GameplayStatics.GetPlayerController` 0)))))

(event `self.ReceiveActorEndOverlap`
  (params (OtherActor :type "Actor Object Reference"))
  (`/Game/DES250_Macros.PlayerCheck` OtherActor
    (:`IsPlayer`
      (`SceneComponent.SetVisibility` (`self.FrontWidget`) false false)
      (`self.DisableInput` (`GameplayStatics.GetPlayerController` 0)))))

(fn `OpenDoor`
  (`GameplayStatics.PlaySound2D` "/Game/DoNotChange/PrototypingAssets/Sounds/GeneralFeedback/DES_SFX_Powerup_01.DES_SFX_Powerup_01" 1.0 1.0 0.0 null null)
  (`SceneComponent.SetHiddenInGame` (`self.TriggerCollider`) true false)
  (bind _component (`/Game/DES250_Macros.GetInventory`)
    (:`Is Valid`
      (`/Game/ActorComponents/AC_Inventory.LoseKey` _component))
    (:`Is Not Valid`
      _))
  (`SceneComponent.SetHiddenInGame` (`self.FrontWidget`) true false)
  (`PrimitiveComponent.SetCollisionEnabled` (`self.DoorFrame`) "NoCollision"))

(fn `PlayerHasKey`
  (returns (HasKey :type Boolean))
  (bind _component (`/Game/DES250_Macros.GetInventory`)
    (:`Is Valid`
      (return (`/Game/ActorComponents/AC_Inventory.HasKey` _component)))
    (:`Is Not Valid`
      (return false))))

(fn `UserConstructionScript`)