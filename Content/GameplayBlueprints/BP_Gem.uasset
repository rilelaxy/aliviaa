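; BP_Gem is a collectible gem that adds itself to the inventory of any overlapping actor that has an AC_Inventory component.
; On pickup it calls GainGem on that component, plays a blip sound, and runs a timeline that scales the gem while moving it along its local Z axis.
; When the timeline finishes, NewFunction destroys the gem; overlaps without the component only print a debug failure message.
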(event `self.ReceiveActorBeginOverlap`
  (params (OtherActor :type "Actor Object Reference"))
  (bind _returnvalue (`self.GetComponentByClass` OtherActor "/Game/ActorComponents/AC_Inventory.AC_Inventory_C"))
  (`/Engine/EditorBlueprintResources/StandardMacros.IsValid` _returnvalue
    (:`Is Valid`
      (`/Game/ActorComponents/AC_Inventory.GainGem` _returnvalue)
      (`GameplayStatics.PlaySoundAtLocation` "/Game/DoNotChange/PrototypingAssets/Sounds/GeneralFeedback/DES_SFX_Blip_03.DES_SFX_Blip_03" (`self.K2_GetActorLocation`) (struct) 1.0 1.0 0.0 null null null null)
      (bind (_direction _newtrack_1) (`Timeline|Timeline`)
        (:`Update`
          (`self.SetActorScale3D` (`KismetMathLibrary.MakeVector` _newtrack_1 _newtrack_1 _newtrack_1))
          (`self.K2_AddActorLocalOffset` (0.0 0.0 3.0)))
        (:`Finished`
          (`self.NewFunction`))))
    (:`Is Not Valid`
      (`KismetSystemLibrary.PrintString` "CAST FAILED" true true (struct :`R` 1.0 :`B` 0.445455 :`A` 1.0)))))

(fn `NewFunction`
  (`self.K2_DestroyActor`))

(fn `UserConstructionScript`)