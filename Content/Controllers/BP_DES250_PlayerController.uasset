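; Player controller that runs pause, win and lose flow for the game and provides debug keys for testing health, lives and inventory.
; On possession it caches the pawn's health and inventory components, which the debug keys drive alongside respawn-point setting and forced win or loss.
; Escape toggles a pause menu created at BeginPlay, blocked once the game is over.
; Win and lose pause, hide the HUD and show one game-over widget page each.
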(event EventPossess
  (params (PossessedPawn :type Pawn%20Object%20Reference))
  (Variables|Default|SetPlayerHealth (Actor|GetComponentbyClass PossessedPawn "/Game/ActorComponents/AC_Health.AC_Health_C"))
  (Variables|Default|SetPlayerInventory (Actor|GetComponentbyClass PossessedPawn "/Game/ActorComponents/AC_Inventory.AC_Inventory_C")))

(event EventBeginPlay
  (bind _returnvalue (UserInterface|CreateWidget "/Game/UI/WBP_PauseMenu.WBP_PauseMenu_C"))
  (Variables|Default|SetPauseMenu _returnvalue))

(event Input|KeyboardEvents|DebugKeyV
  (params (Key :type Key%20Structure) (ActionValue :type Input%20Action%20Value%20Structure))
  (:Pressed
    (CallFunction|WinGame)))

(event Input|KeyboardEvents|DebugKeyK
  (params (Key :type Key%20Structure) (ActionValue :type Input%20Action%20Value%20Structure))
  (:Pressed
    (CallFunction|LoseGame)))

(event Input|KeyboardEvents|DebugKey2
  (params (Key :type Key%20Structure) (ActionValue :type Input%20Action%20Value%20Structure))
  (:Pressed
    (Default|LoseCoin (Variables|Default|GetPlayerInventory))))

(event Input|KeyboardEvents|DebugKey3
  (params (Key :type Key%20Structure) (ActionValue :type Input%20Action%20Value%20Structure))
  (:Pressed
    (Default|GainGem (Variables|Default|GetPlayerInventory))))

(event Input|KeyboardEvents|DebugKey4
  (params (Key :type Key%20Structure) (ActionValue :type Input%20Action%20Value%20Structure))
  (:Pressed
    (Default|LoseGem (Variables|Default|GetPlayerInventory))))

(event Input|KeyboardEvents|DebugKey5
  (params (Key :type Key%20Structure) (ActionValue :type Input%20Action%20Value%20Structure))
  (bind _playerinventory (Variables|Default|GetPlayerInventory))
  (:Pressed
    (Default|GainKey _playerinventory)
    (Variables|/Game/ActorComponents/AC_Inventory.AC_Inventory_C|SetHasKey _playerinventory true)))

(event Input|KeyboardEvents|DebugKey6
  (params (Key :type Key%20Structure) (ActionValue :type Input%20Action%20Value%20Structure))
  (bind _playerinventory (Variables|Default|GetPlayerInventory))
  (:Pressed
    (Default|LoseKey _playerinventory)
    (Variables|/Game/ActorComponents/AC_Inventory.AC_Inventory_C|SetHasKey _playerinventory false)))

(event Input|KeyboardEvents|DebugKeyV
  (params (Key :type Key%20Structure) (ActionValue :type Input%20Action%20Value%20Structure))
  (:Pressed
    (CallFunction|WinGame)))

(event Input|KeyboardEvents|DebugKeyJ
  (params (Key :type Key%20Structure) (ActionValue :type Input%20Action%20Value%20Structure))
  (:Pressed
    (Default|TakeDamage (Variables|Default|GetPlayerHealth) 1e+01)))

(event Input|KeyboardEvents|DebugKeyH
  (params (Key :type Key%20Structure) (ActionValue :type Input%20Action%20Value%20Structure))
  (:Pressed
    (Default|Heal (Variables|Default|GetPlayerHealth) 1e+01)))

(event Input|KeyboardEvents|DebugKeyL
  (params (Key :type Key%20Structure) (ActionValue :type Input%20Action%20Value%20Structure))
  (:Pressed
    (Default|LoseLife (Variables|Default|GetPlayerHealth))))

(event Input|KeyboardEvents|DebugKeySemicolon
  (params (Key :type Key%20Structure) (ActionValue :type Input%20Action%20Value%20Structure))
  (:Pressed
    (Default|GainLife (Variables|Default|GetPlayerHealth))))

(event Input|KeyboardEvents|DebugKeyP
  (params (Key :type Key%20Structure) (ActionValue :type Input%20Action%20Value%20Structure))
  (bind _returnvalue (Game|Player|GetPlayerPawn 0))
  (bind _returnvalue_2 (Actor|GetComponentbyClass _returnvalue "/Game/ActorComponents/AC_Health.AC_Health_C"))
  (:Pressed
    (Variables|/Game/ActorComponents/AC_Health.AC_Health_C|SetRespawnLocation _returnvalue_2 (Transformation|GetActorLocation))
    (Variables|/Game/ActorComponents/AC_Health.AC_Health_C|SetRespawnRotation _returnvalue_2 (Transformation|GetActorRotation))))

(event Input|KeyboardEvents|DebugKey6
  (params (Key :type Key%20Structure) (ActionValue :type Input%20Action%20Value%20Structure))
  (:Pressed
    (Default|LoseKey (Variables|Default|GetPlayerInventory))
    (if true
      (Audio|PlaySound2D "/Game/DoNotChange/PrototypingAssets/Sounds/GeneralFeedback/DES_SFX_Random_02.DES_SFX_Random_02" 1.0 1.0 0.0 0 0)
      (else
        (Audio|PlaySound2D "/Game/DoNotChange/PrototypingAssets/Sounds/GeneralFeedback/DES_SFX_Random_03.DES_SFX_Random_03" 1.0 1.0 0.0 0 0)))))

(event Input|KeyboardEvents|DebugKey5
  (params (Key :type Key%20Structure) (ActionValue :type Input%20Action%20Value%20Structure))
  (:Pressed
    (Default|GainKey (Variables|Default|GetPlayerInventory))
    (Audio|PlaySound2D "/Game/DoNotChange/PrototypingAssets/Sounds/GeneralFeedback/DES_SFX_Random_01.DES_SFX_Random_01" 1.0 1.0 0.0 0 0)))

(event Input|KeyboardEvents|DebugKey1
  (params (Key :type Key%20Structure) (ActionValue :type Input%20Action%20Value%20Structure))
  (:Pressed
    (Default|GainCoin (Variables|Default|GetPlayerInventory))))

(event Input|KeyboardEvents|Escape
  (params (Key :type Key%20Structure))
  (:Pressed
    (if (Game|IsGamePaused)
      (CallFunction|ResumeGame)
      (else
        (CallFunction|Pausing)))))

(fn ConstructionScript)

(fn Pausing
  (if (not (Variables|Default|GetIsGameOver))
    ;[0.15 0.15 0.15 0.5] Comment
    (Audio|PlaySound2D "/Game/DoNotChange/PrototypingAssets/Sounds/GeneralFeedback/DES_SFX_Bounce_01.DES_SFX_Bounce_01" 1.0 1.0 0.0 0 0)
    (UserInterface|Viewport|AddtoViewport (Variables|Default|GetPauseMenu) 0)
    (Game|SetGamePaused true)
    (Variables|Default|SetbShowMouseCursor true)
    (Input|SetInputModeGameandUI self (Variables|Default|GetPauseMenu) "DoNotLock" true false)))

(fn ResumeGame
  (if (not (Variables|Default|GetIsGameOver))
    (Audio|PlaySound2D "/Game/DoNotChange/PrototypingAssets/Sounds/GeneralFeedback/DES_SFX_Bell_01.DES_SFX_Bell_01" 1.0 1.0 0.0 0 0)
    (Game|SetGamePaused false)
    (Widget|RemovefromParent (Variables|Default|GetPauseMenu))
    (Variables|Default|SetbShowMouseCursor false)
    (Input|SetInputModeGameOnly self true)))

(fn WinGame
  (Game|SetGamePaused true)
  (Audio|PlaySound2D "/Game/DoNotChange/PrototypingAssets/Sounds/GameStateChanges/DES_Stinger_Happy_02.DES_Stinger_Happy_02" 1.0 1.0 0.0 0 0)
  (bind _asbi_player_character (Utilities|Casting|CastToBI_PlayerCharacter (Pawn|GetControlledPawn)))
  (Default|HideHud _asbi_player_character)
  (bind _returnvalue (UserInterface|CreateWidget "/Game/UI/WBP_GameOver.WBP_GameOver_C"))
  (Class|WidgetSwitcher|SetActiveWidgetIndex (Variables|/Game/UI/WBP_GameOver.WBP_GameOver_C|GetWidgetSwitcher _returnvalue))
  (UserInterface|Viewport|AddtoViewport _returnvalue 0)
  (Variables|Default|SetIsGameOver true)
  (Variables|Default|SetbShowMouseCursor true)
  (Input|SetInputModeUIOnly (Game|GetPlayerController 0) _returnvalue "DoNotLock" false))

(fn LoseGame
  (Game|SetGamePaused true)
  (Audio|PlaySound2D "/Game/DoNotChange/PrototypingAssets/Sounds/GameStateChanges/DES_Stinger_Sad_02.DES_Stinger_Sad_02" 1.0 1.0 0.0 0 0)
  (bind _asbi_player_character (Utilities|Casting|CastToBI_PlayerCharacter (Pawn|GetControlledPawn)))
  (Default|HideHud _asbi_player_character)
  (bind _returnvalue (UserInterface|CreateWidget "/Game/UI/WBP_GameOver.WBP_GameOver_C"))
  (Class|WidgetSwitcher|SetActiveWidgetIndex (Variables|/Game/UI/WBP_GameOver.WBP_GameOver_C|GetWidgetSwitcher _returnvalue) 1)
  (UserInterface|Viewport|AddtoViewport _returnvalue 0)
  (Variables|Default|SetIsGameOver true)
  (Variables|Default|SetbShowMouseCursor true)
  (Input|SetInputModeUIOnly (Game|GetPlayerController 0) _returnvalue "DoNotLock" false))