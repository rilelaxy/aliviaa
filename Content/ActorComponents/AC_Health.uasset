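; AC_Health is an actor component that manages its owner's health and lives, with sound feedback for damage, healing and life changes.
; It records the owner's starting transform on BeginPlay as the respawn point.
; Depleted health costs a life, then either refills health and teleports the owner back, resetting player 0's control rotation, or calls LoseGame on BP_DES250_PlayerController.
; Heal clamps to max health and returns whether healing applied.
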(event `self.ReceiveBeginPlay`
  (bind _returnvalue (`self.GetOwner`))
  (set `self.RespawnLocation` (`Actor.K2_GetActorLocation` _returnvalue))
  (set `self.RespawnRotation` (`Actor.K2_GetActorRotation` _returnvalue)))

(fn `GainLife`
  (bind _currentlives (`self.CurrentLives`))
  (if (> _currentlives 0)
    (`/Engine/EditorBlueprintResources/StandardMacros.IncrementInt` _currentlives
      (:`  `
        (`GameplayStatics.PlaySound2D` "/Game/DoNotChange/PrototypingAssets/Sounds/GeneralFeedback/DES_SFX_Jump_02.DES_SFX_Jump_02" 1.0 1.0 0.0 null null)))))

(fn `GetPercent`
  (returns (Percent :type "Float (double-precision)"))
  (return (/ (`self.CurrentHealth`) (`self.MaxHealth`))))

(fn `Heal`
  (params (B :type "Float (double-precision)"))
  (returns (`Was Healed` :type Boolean))
  (bind _currenthealth (`self.CurrentHealth`))
  (bind _output_get (set `self.WasHealed` (< _currenthealth (`self.MaxHealth`))))
  (if _output_get
    (set `self.CurrentHealth` (`KismetMathLibrary.FClamp` (+ _currenthealth B) 0.0 (`self.MaxHealth`)))
    (`GameplayStatics.PlaySound2D` "/Game/DoNotChange/PrototypingAssets/Sounds/GeneralFeedback/DES_SFX_Powerup_04.DES_SFX_Powerup_04" 1.0 1.0 0.0 null null))
  (return (`self.WasHealed`)))

(fn `LoseLife`
  (bind _result (`/Engine/EditorBlueprintResources/StandardMacros.DecrementInt` (`self.CurrentLives`))
    (:`  `
      (if (> _result 0)
        (`GameplayStatics.PlaySound2D` "/Game/DoNotChange/PrototypingAssets/Sounds/GeneralFeedback/DES_SFX_Diminuendo_01.DES_SFX_Diminuendo_01" 1.0 1.0 0.0 null null)
        (set `self.CurrentHealth` (`self.MaxHealth`))
        (`Actor.K2_SetActorLocation` (`self.GetOwner`) (`self.RespawnLocation`) false true)
        (`Controller.SetControlRotation` (`GameplayStatics.GetPlayerController` 0) (`self.RespawnRotation`))
        (else
          (bind _asbp_des250_player_controller (cast `/Game/Controllers/BP_DES250_PlayerController` (`GameplayStatics.GetPlayerController` 0)))
          (`/Game/Controllers/BP_DES250_PlayerController.LoseGame` _asbp_des250_player_controller))))))

(fn `TakeDamage`
  (params (Amount :type "Float (double-precision)" :default 1.0))
  (if true
    (bind _output_get (set `self.CurrentHealth` (- (`self.CurrentHealth`) Amount)))
    (`GameplayStatics.PlaySound2D` "/Game/DoNotChange/PrototypingAssets/Sounds/GeneralFeedback/DES_SFX_Powerup_01.DES_SFX_Powerup_01" 1.0 1.0 0.0 null null)
    (if (<= _output_get 0.0)
      (`self.LoseLife`))))