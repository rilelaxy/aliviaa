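; AC_Inventory is an inventory component that tracks a coin count, a gem count and whether a key is held.
; Gain functions increment the coin and gem counters or set the key flag.
; LoseKey clears the flag and returns whether a key was held, while LoseCoin and LoseGem are empty stubs.
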(fn `GainCoin`
  (`/Engine/EditorBlueprintResources/StandardMacros.IncrementInt` (`self.CoinCount`)))

(fn `GainGem`
  (`/Engine/EditorBlueprintResources/StandardMacros.IncrementInt` (`self.GemCount`)))

(fn `GainKey`
  (set `self.HasKey` true))

(fn `LoseCoin`)

(fn `LoseGem`)

(fn `LoseKey`
  (returns (ConsumedKey :type Boolean))
  (if (`self.HasKey`)
    (set `self.HasKey` false)
    (return true)
    (else
      (return false))))